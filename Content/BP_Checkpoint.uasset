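; BP_Checkpoint is a trigger-based checkpoint for the motion matching player character.
; When that character overlaps the trigger, the checkpoint registers itself as LastCheckpoint on BP_ThirdPersonGameMode and plays a 2D sound.
; It then resets the HUD countdown timer through the game mode's player HUD reference.
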(event OnComponentBeginOverlap(Trigger)
  (params (OverlappedComponent :type Primitive%20Component%20Object%20Reference) (OtherActor :type Actor%20Object%20Reference) (OtherComp :type Primitive%20Component%20Object%20Reference) (OtherBodyIndex :type Integer) (bFromSweep :type Boolean) (SweepResult :type Hit%20Result%20Structure%20%28by%20ref%29))
  (Utilities|Casting|CastToBP_MotionMatchingCharacter OtherActor)
  (bind _asbp_third_person_game_mode (Utilities|Casting|CastToBP_ThirdPersonGameMode (Game|GetGameMode)))
  (Variables|/Game/ThirdPerson/Blueprints/BP_ThirdPersonGameMode.BP_ThirdPersonGameMode_C|SetlastCheckpoint _asbp_third_person_game_mode self)
  (Audio|PlaySound2D "/Game/StarterContent/Audio/Collapse01.Collapse01" 1.0 1.0 0.0 0 0)
  (bind _asbp_third_person_game_mode_2 (Utilities|Casting|CastToBP_ThirdPersonGameMode (Game|GetGameMode)))
  (Default|ResetCountdown (Variables|/Game/PlayerInGameHUD.PlayerInGameHUD_C|GetCountdownTimerRef (Variables|/Game/ThirdPerson/Blueprints/BP_ThirdPersonGameMode.BP_ThirdPersonGameMode_C|GetPlayerHUDRef _asbp_third_person_game_mode_2))))

(fn ConstructionScript)